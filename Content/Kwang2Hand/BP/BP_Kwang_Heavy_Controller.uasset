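; Click-to-move player controller for the Kwang Heavy character, handling movement and attack clicks from the cursor hit point.
; Holding MoveHold repaths toward the cursor every tick through a gate, skipping points too near the pawn and spawning a click effect.
; Attack turns toward the target, paths to it and requests an attack-range move on Kwang_Heavy_BP.
; Tick stops movement within range and rotates the pawn's yaw at TurnRate until aligned.
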(event `self.ReceiveBeginPlay`)

(event `InputAction|MoveHold`
  (params (Key :type "Key Structure"))
  (:`Pressed`
    (goto _label :!via `Open`))
  (:`Released`
    (goto _label :!via `Close`)))

(event `self.ReceiveTick`
  (params (DeltaSeconds :type "Float (single-precision)"))
  (`|ExecutionSequence`
    (:`then_0`
      (`/Engine/EditorBlueprintResources/StandardMacros.Gate` true :!label _label ; While key is pressed...
        (:`Exit`
          (`self.MoveToHitLocation` (`.Location` (`GameplayStatics.BreakHitResult` (`self.GetHitResultUnderCursorByChannel` "TraceTypeQuery1")))) ; ..and move there.
        )))
    (:`then_1`
      (`self.CheckPathFindingRange`))
    (:`then_2`
      (`self.CheckLookAtAngle` DeltaSeconds))))

(event `InputAction|Attack`
  (params (Key :type "Key Structure"))
  (bind (_bblockinghit _binitialoverlap _time _distance _location) (`GameplayStatics.BreakHitResult` (`self.GetHitResultUnderCursorByChannel` "TraceTypeQuery1")))
  (:`Pressed`
    (`self.TurnToHitLocation` _location)
    (`self.MoveToHitLocationWithRange` 200.0 _location)))

(fn `CheckLookAtAngle`
  (params (DeltaTime :type "Float (double-precision)"))
  (bind _returnvalue (`self.K2_GetActorRotation` (`self.K2_GetPawn`)))
  (bind _yaw (.yaw (`KismetMathLibrary.NormalizedDeltaRotator` (`self.TargetAngle`) _returnvalue)))
  (bind _returnvalue_2 (* (`self.TurnRate`) (* (`KismetMathLibrary.SignOfFloat` _yaw) DeltaTime)))
  (if (`self.CheckingLookAtAngle`)
    (if (< (`KismetMathLibrary.Abs` _yaw) (`KismetMathLibrary.Abs` (.yaw _returnvalue_2)))
      (`self.K2_SetActorRotation` (`self.K2_GetPawn`) (`self.TargetAngle`) false)
      (set `self.CheckingLookAtAngle` false)
      (else
        (`self.K2_SetActorRotation` (`self.K2_GetPawn`) (`KismetMathLibrary.ComposeRotators` _returnvalue _returnvalue_2) false)))))

(fn `CheckPathFindingRange`
  (if (`self.CheckingPathFindingRange`)
    (if (<= (`KismetMathLibrary.VSize` (- (`self.PathFindingDestination`) (`self.K2_GetActorLocation` (`self.K2_GetPawn`)))) (`self.PathFindingAcceptanceRange`))
      (`self.StopMovement`)
      (set `self.CheckingPathFindingRange` false))))

(fn `MoveToHitLocation`
  (params (Position :type "Vector Structure"))
  (if (>= (`KismetMathLibrary.VSize` (- (`self.K2_GetActorLocation` (`self.K2_GetPawn`)) Position)) (`self.MinClickDistance`))
    (`AIBlueprintHelperLibrary.SimpleMoveToLocation` self Position)
    (`GameplayStatics.SpawnEmitterAtLocation` "/Game/LinhiBlade/MouseClickParticle/P_MouseClick.P_MouseClick" Position (struct :`Roll` 90.0) (1.0 1.0 1.0) true "AutoRelease")))

(fn `MoveToHitLocationWithRange`
  (params (Range :type "Float (double-precision)") (Destination :type "Vector Structure"))
  (set `self.CheckingPathFindingRange` true)
  (set `self.PathFindingAcceptanceRange` Range)
  (set `self.PathFindingDestination` Destination)
  (`self.MoveToHitLocation` Destination)
  (bind _askwang_heavy_bp (cast `/Game/Kwang2Hand/BP/Kwang_Heavy_BP` (`self.K2_GetPawn`)))
  (`/Game/Kwang2Hand/BP/Kwang_Heavy_BP.RequestMoveToAttackRange` _askwang_heavy_bp (`self.PathFindingDestination`) (`self.PathFindingAcceptanceRange`)))

(fn `TurnToHitLocation`
  (params (Position :type "Vector Structure"))
  (set `self.CheckingLookAtAngle` true)
  (set `self.TargetAngle` (`KismetMathLibrary.MakeRotator` 0.0 0.0 (.yaw (`KismetMathLibrary.FindLookAtRotation` (`self.K2_GetActorLocation` (`self.K2_GetPawn`)) Position)))))

(fn `UserConstructionScript`)