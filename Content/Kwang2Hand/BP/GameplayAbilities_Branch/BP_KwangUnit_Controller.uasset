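; Player controller that drives a separate Kwang hero unit with click-to-move and ability input while the possessed pawn serves as the camera.
; Camera axes add movement input to the pawn along its right and forward vectors.
; MoveHold sends the ControlledUnit's AIController to the cursor hit location and spawns a click effect.
; Q activates the hero's first ability slot, and the left and right mouse buttons confirm or cancel targeting.
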(event `self.ReceiveBeginPlay`)

(event `InputAxis|CameraX`
  (params (AxisValue :type "Float (single-precision)"))
  (bind _returnvalue (`self.K2_GetPawn`))
  (`Pawn.AddMovementInput` _returnvalue (`SceneComponent.GetRightVector` (`Actor.RootComponent` _returnvalue)) AxisValue false))

(event `self.ReceiveTick`
  (params (DeltaSeconds :type "Float (single-precision)")))

(event `InputAxis|CameraY`
  (params (AxisValue :type "Float (single-precision)"))
  (bind _returnvalue (`self.K2_GetPawn`))
  (`Pawn.AddMovementInput` _returnvalue (`SceneComponent.GetForwardVector` (`Actor.RootComponent` _returnvalue)) AxisValue false))

(event `InputAction|MoveHold`
  (params (Key :type "Key Structure"))
  (bind (_bblockinghit _binitialoverlap _time _distance _location) (`GameplayStatics.BreakHitResult` (`self.GetHitResultUnderCursorByChannel` "TraceTypeQuery1")))
  (:`Pressed`
    (bind _asaicontroller (cast `AIController` (`Pawn.GetController` (`self.ControlledUnit`))))
    (`AIController.MoveToLocation` _asaicontroller _location -1.0 true true false true null true)
    (`GameplayStatics.SpawnEmitterAtLocation` "/Game/LinhiBlade/MouseClickParticle/P_MouseClick.P_MouseClick" _location (struct :`Roll` 90.0) (1.0 1.0 1.0) true "AutoRelease")))

(event `Key|Q`
  (params (Key :type "Key Structure"))
  (:`Pressed`
    (bind _askwang_hero (cast `/Game/Kwang2Hand/BP/GameplayAbilities_Branch/Abilities/KwangHero` (`self.ControlledUnit`)))
    (`AP_Hero.ActivateAbilitySlot` _askwang_hero 0 true)))

(event `Key|LeftMouseButton`
  (params (Key :type "Key Structure"))
  (:`Pressed`
    (bind _askwang_hero (cast `/Game/Kwang2Hand/BP/GameplayAbilities_Branch/Abilities/KwangHero` (`self.ControlledUnit`)))
    (`/Game/Kwang2Hand/BP/GameplayAbilities_Branch/Abilities/KwangHero.TargetConfirm` _askwang_hero)))

(event `Key|RightMouseButton`
  (params (Key :type "Key Structure"))
  (:`Pressed`
    (bind _askwang_hero (cast `/Game/Kwang2Hand/BP/GameplayAbilities_Branch/Abilities/KwangHero` (`self.ControlledUnit`)))
    (`/Game/Kwang2Hand/BP/GameplayAbilities_Branch/Abilities/KwangHero.TargetCancel` _askwang_hero)))

(fn `UserConstructionScript`)