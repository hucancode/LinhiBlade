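; Player controller for MOBA-style play, steering a camera pawn while commanding a separate AI-controlled KwangHero unit.
; Camera axes move the pawn, and MoveHold sends the unit's AIController to the cursor hit location with a click effect.
; Ability inputs activate hero slots through UseAbility and set a Targeting flag, which blocks move orders until confirm or cancel clears it.
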(event `self.ReceiveBeginPlay`)

(event `InputAxis|CameraX`
  (params (AxisValue :type "Float (single-precision)"))
  (bind _returnvalue (`self.K2_GetPawn`))
  (`Pawn.AddMovementInput` _returnvalue (`SceneComponent.GetRightVector` (`Actor.RootComponent` _returnvalue)) AxisValue false))

(event `self.ReceiveTick`
  (params (DeltaSeconds :type "Float (single-precision)")))

(event `InputAxis|CameraY`
  (params (AxisValue :type "Float (single-precision)"))
  (bind _returnvalue (`self.K2_GetPawn`))
  (`Pawn.AddMovementInput` _returnvalue (`SceneComponent.GetForwardVector` (`Actor.RootComponent` _returnvalue)) AxisValue false))

(event `InputAction|MoveHold`
  (params (Key :type "Key Structure"))
  (bind (_bblockinghit _binitialoverlap _time _distance _location) (`GameplayStatics.BreakHitResult` (`self.GetHitResultUnderCursorByChannel` "TraceTypeQuery1")))
  (:`Pressed`
    (if (not (`self.Targeting`))
      (bind _asaicontroller (cast `AIController` (`Pawn.GetController` (`self.ControlledUnit`))))
      (`AIController.MoveToLocation` _asaicontroller _location -1.0 true true false true null true)
      (`GameplayStatics.SpawnEmitterAtLocation` "/Game/LinhiBlade/MouseClickParticle/P_MouseClick.P_MouseClick" _location (struct :`Roll` 90.0) (1.0 1.0 1.0) true "AutoRelease"))))

(event `InputAction|WeaponAbility`
  (params (Key :type "Key Structure"))
  (:`Pressed`
    (`self.UseAbility` 0)))

(event `InputAction|ConfirmAbility`
  (params (Key :type "Key Structure"))
  (:`Pressed`
    (bind _askwang_hero (cast `/Game/Kwang2Hand/BP/GameplayAbilities_Branch/Abilities/KwangHero` (`self.ControlledUnit`)))
    (`/Game/Kwang2Hand/BP/GameplayAbilities_Branch/Abilities/KwangHero.TargetConfirm` _askwang_hero)
    (set `self.Targeting` false :!label _label)))

(event `InputAction|UseAbility1`
  (params (Key :type "Key Structure"))
  (:`Pressed`
    (`self.UseAbility` 1)))

(event `InputAction|UseAbility2`
  (params (Key :type "Key Structure"))
  (:`Pressed`
    (`self.UseAbility` 2)))

(event `InputAction|UseAbility3`
  (params (Key :type "Key Structure"))
  (:`Pressed`
    (`self.UseAbility` 3)))

(event `InputAction|CancelAbility`
  (params (Key :type "Key Structure"))
  (:`Pressed`
    (bind _askwang_hero (cast `/Game/Kwang2Hand/BP/GameplayAbilities_Branch/Abilities/KwangHero` (`self.ControlledUnit`)))
    (`/Game/Kwang2Hand/BP/GameplayAbilities_Branch/Abilities/KwangHero.TargetCancel` _askwang_hero)
    (goto _label)))

(event `InputAction|UseAbility4`
  (params (Key :type "Key Structure"))
  (:`Pressed`
    (`self.UseAbility` 4)))

(event `InputAction|UseAbility5`
  (params (Key :type "Key Structure"))
  (:`Pressed`
    (`self.UseAbility` 5)))

(event `InputAction|UseAbility6`
  (params (Key :type "Key Structure"))
  (:`Pressed`
    (`self.UseAbility` 6)))

(fn `UseAbility`
  (params (AbilitySlot :type Integer))
  (bind _askwang_hero (cast `/Game/Kwang2Hand/BP/GameplayAbilities_Branch/Abilities/KwangHero` (`self.ControlledUnit`)))
  (`AP_Hero.ActivateAbilitySlot` _askwang_hero AbilitySlot true)
  (set `self.Targeting` true))

(fn `UserConstructionScript`)