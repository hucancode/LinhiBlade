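; Kwang heavy character Blueprint that drives a buffered four-step attack combo and forwards jump and cancel input to its Anim Blueprint.
; RequestMoveToAttackRange stores a destination, and Tick triggers RequestAttack once distance and facing yaw are within tolerance.
; An attack requested mid-swing is saved, then played on the Anim Blueprint's proxy-hit event as the next cycling index.
; The attack-exit event resets the combo.
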(event `InputAction|Jump`
  (params (Key :type "Key Structure"))
  (:`Pressed`
    (`self.RequestJump`)))

(event `InputAction|Stop`
  (params (Key :type "Key Structure"))
  (:`Pressed`
    (`self.RequestCancel`)))

(event `InputAction|Attack`
  (params (Key :type "Key Structure")))

(event `self.ReceiveBeginPlay`
  (bind _askwang_heavy_anim_bp (cast `/Game/Kwang2Hand/BP/Kwang_Heavy_Anim_BP` (`SkeletalMeshComponent.GetAnimInstance` (`self.Mesh`))))
  (bind _output_get (set `self.AnimBlueprint` _askwang_heavy_anim_bp))
  (add `/Game/Kwang2Hand/BP/Kwang_Heavy_Anim_BP.OnAttackExit` _output_get (delegate `OnAttackExit`))
  (add `/Game/Kwang2Hand/BP/Kwang_Heavy_Anim_BP.OnAttackProxyHit` _output_get (delegate `OnAttackProxyHit`)))

(event `OnAttackExit`
  (`self.ExitAttackMode`))

(event `self.ReceiveTick`
  (params (DeltaSeconds :type "Float (single-precision)"))
  (`self.CheckAttackRange`))

(event `OnAttackProxyHit`
  (`self.RevokeSavedAttack`))

(fn `CalculateNextAttack`
  (set `self.CurrentAttack` (mod (+ (`self.CurrentAttack`) 1) 4)))

(fn `CheckAttackRange`
  (if (`self.IsGettingInAttackRange`)
    (if true
      (if (and (<= (`KismetMathLibrary.VSize` (- (`self.AttackDestination`) (`self.K2_GetActorLocation`))) (`self.AttackAcceptanceRange`)) (< (`KismetMathLibrary.Abs` (.yaw (`KismetMathLibrary.NormalizedDeltaRotator` (`KismetMathLibrary.FindLookAtRotation` (`self.K2_GetActorLocation`) (`self.AttackDestination`)) (`self.K2_GetActorRotation`)))) (`self.AttackAcceptanceAngle`)))
        (set `self.IsGettingInAttackRange` false)
        (`self.RequestAttack`)))))

(fn `ExitAttackMode`
  (set `self.IsAttacking` false)
  (set `self.IsSavingAttack` false)
  (set `self.CurrentAttack` -1))

(fn `RequestAttack`
  (if (`self.IsAttacking`)
    (if (not (`self.IsSavingAttack`))
      (set `self.IsSavingAttack` true))
    (else
      (set `self.IsAttacking` true)
      (`self.CalculateNextAttack`)
      (`/Game/Kwang2Hand/BP/Kwang_Heavy_Anim_BP.RequestAttack` (`self.AnimBlueprint`) (`self.CurrentAttack`))))
  (return))

(fn `RequestCancel`
  (`/Game/Kwang2Hand/BP/Kwang_Heavy_Anim_BP.RequestCancel` (`self.AnimBlueprint`)))

(fn `RequestJump`
  (`/Game/Kwang2Hand/BP/Kwang_Heavy_Anim_BP.RequestJump` (`self.AnimBlueprint`)))

(fn `RequestMoveToAttackRange`
  (params (Destination :type "Vector Structure") (AcceptanceRange :type "Float (double-precision)"))
  (set `self.IsGettingInAttackRange` true)
  (set `self.AttackDestination` Destination)
  (set `self.AttackAcceptanceRange` AcceptanceRange))

(fn `RevokeSavedAttack`
  (if (`self.IsSavingAttack`)
    (set `self.IsSavingAttack` false)
    (set `self.IsAttacking` true)
    (`self.CalculateNextAttack`)
    (`/Game/Kwang2Hand/BP/Kwang_Heavy_Anim_BP.RequestAttack` (`self.AnimBlueprint`) (`self.CurrentAttack`))))

(fn `TurnToPosition`
  (params (Position :type "Vector Structure"))
  (`self.K2_SetActorRotation` (`KismetMathLibrary.MakeRotator` 0.0 0.0 (.yaw (`KismetMathLibrary.FindLookAtRotation` (`self.K2_GetActorLocation`) Position)))))

(fn `UserConstructionScript`)