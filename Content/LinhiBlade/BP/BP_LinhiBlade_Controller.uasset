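; Player controller for LinhiBlade that drives click-to-move and attack-approach movement from the cursor.
; While MoveHold or Attack is held, Tick-fed gates trace under the cursor and path the pawn there via SimpleMoveToLocation with a click effect.
; Attack also yaws the pawn toward the point and stores a range that Tick checks to stop movement.
; That range flag is never cleared, and no attack action is triggered here.
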(event `self.ReceiveBeginPlay`)

(event `InputAction|MoveHold`
  (params (Key :type "Key Structure"))
  (:`Pressed`
    (goto _label :!via `Open`))
  (:`Released`
    (goto _label :!via `Close`)))

(event `InputAction|Attack` :consume false
  (params (Key :type "Key Structure"))
  (bind (_bblockinghit _binitialoverlap _time _distance _location) (`GameplayStatics.BreakHitResult` (`self.GetHitResultUnderCursorByChannel` "TraceTypeQuery1")))
  (:`Pressed`
    (goto _label_2 :!via `Open`))
  (:`Released`
    (goto _label_2 :!via `Close`)))

(event `self.ReceiveTick`
  (params (DeltaSeconds :type "Float (single-precision)"))
  (bind (_bblockinghit _binitialoverlap _time _distance _location) (`GameplayStatics.BreakHitResult` (`self.GetHitResultUnderCursorByChannel` "TraceTypeQuery1")))
  (`|ExecutionSequence`
    (:`then_0`
      (`/Engine/EditorBlueprintResources/StandardMacros.Gate` true :!label _label ; While key is pressed...
        (:`Exit`
          (`self.MoveToHitLocation` _location) ; ..and move there.
        )))
    (:`then_1`
      (`/Engine/EditorBlueprintResources/StandardMacros.Gate` true :!label _label_2 ; While key is pressed...
        (:`Exit`
          (`self.TurnToHitLocation` _location)
          (`self.MoveToHitLocationWithRange` 200.0 _location))))
    (:`then_2`
      (`self.CheckPathFindingRange`))))

(fn `CheckPathFindingRange`
  (if (`self.PathFindingWithRange`)
    (if (<= (`KismetMathLibrary.VSize` (- (`self.PathFindingDestination`) (`self.K2_GetActorLocation` (`self.K2_GetPawn`)))) (`self.PathFindingAcceptanceRange`))
      (`self.StopMovement`))))

(fn `MoveToHitLocation`
  (params (Position :type "Vector Structure"))
  (if (>= (`KismetMathLibrary.VSize` (- (`self.K2_GetActorLocation` (`self.K2_GetPawn`)) Position)) (`self.MinClickDistance`))
    (`AIBlueprintHelperLibrary.SimpleMoveToLocation` self Position)
    (`GameplayStatics.SpawnEmitterAtLocation` "/Game/LinhiBlade/MouseClickParticle/P_MouseClick.P_MouseClick" Position (struct :`Roll` 90.0) (1.0 1.0 1.0) true "AutoRelease")))

(fn `MoveToHitLocationWithRange`
  (params (Range :type "Float (double-precision)") (Destination :type "Vector Structure"))
  (set `self.PathFindingWithRange` true)
  (set `self.PathFindingAcceptanceRange` Range)
  (set `self.PathFindingDestination` Destination)
  (`self.MoveToHitLocation` Destination))

(fn `TurnToHitLocation`
  (params (Position :type "Vector Structure"))
  (bind _returnvalue (`self.K2_GetPawn`))
  (`self.K2_SetActorRotation` _returnvalue (`KismetMathLibrary.MakeRotator` 0.0 0.0 (.yaw (`KismetMathLibrary.FindLookAtRotation` (`self.K2_GetActorLocation` _returnvalue) Position))) false))

(fn `UserConstructionScript`)