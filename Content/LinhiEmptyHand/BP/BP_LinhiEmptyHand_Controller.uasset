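; BP_LinhiEmptyHand_Controller is a click-to-move player controller that steers its pawn toward the point under the cursor.
; While MoveHold is pressed, a gate lets Tick run a complex Visibility trace under the cursor each frame and pass the hit to MoveToHitLocation.
; That function skips points too close to the pawn, otherwise calls SimpleMoveToLocation and spawns an auto-released click particle there.
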(event `InputAction|MoveHold`
  (params (Key :type "Key Structure"))
  (:`Pressed`
    (goto _label :!via `Open`))
  (:`Released`
    (goto _label :!via `Close`)))

(event `self.ReceiveTick`
  (params (DeltaSeconds :type "Float (single-precision)"))
  (`/Engine/EditorBlueprintResources/StandardMacros.Gate` true :!label _label ; While key is pressed...
    (:`Exit`
      (`self.MoveToHitLocation` (`self.GetHitResultUnderCursorByChannel` "TraceTypeQuery1")) ; ..and move there.
    )))

(fn `MoveToHitLocation`
  (params (Hit :type "HitResult Structure"))
  (bind (_bblockinghit _binitialoverlap _time _distance _location) (`GameplayStatics.BreakHitResult` Hit))
  (if (>= (`KismetMathLibrary.VSize` (- (`self.K2_GetActorLocation` (`self.K2_GetPawn`)) _location)) (`self.MinClickDistance`))
    (`AIBlueprintHelperLibrary.SimpleMoveToLocation` self _location)
    (`GameplayStatics.SpawnEmitterAtLocation` "/Game/LinhiBlade/MouseClickParticle/P_MouseClick.P_MouseClick" _location (struct :`Roll` 90.0) (1.0 1.0 1.0) true "AutoRelease")))

(fn `UserConstructionScript`)